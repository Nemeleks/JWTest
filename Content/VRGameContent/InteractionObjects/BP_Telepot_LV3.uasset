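; VR teleport station actor that presents two portal widgets, each given its own level name.
; On BeginPlay it copies the two level-name variables into each portal's UMG_Teleportation widget.
; A box collision switches the player VR character's interaction drawing on when the player pawn enters and off when it leaves.
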(event `self.ReceiveBeginPlay`
  (bind _asumg_teleportation (cast `/Game/VRGameContent/UI/UMG_Teleportation` (`WidgetComponent.GetUserWidgetObject` (`self.Portal1`))))
  (set `/Game/VRGameContent/UI/UMG_Teleportation.Level Name` (`self.Portal1_LevelName`) _asumg_teleportation)
  (bind _asumg_teleportation_2 (cast `/Game/VRGameContent/UI/UMG_Teleportation` (`WidgetComponent.GetUserWidgetObject` (`self.Portal2`))))
  (set `/Game/VRGameContent/UI/UMG_Teleportation.Level Name` (`self.Portal2_LevelName`) _asumg_teleportation_2))

(event `self.BoxCollision.OnComponentBeginOverlap`
  (params (OverlappedComponent :type "PrimitiveComponent Object Reference") (OtherActor :type "Actor Object Reference") (OtherComp :type "PrimitiveComponent Object Reference") (OtherBodyIndex :type Integer) (bFromSweep :type Boolean) (SweepResult :type "HitResult Structure (by ref)"))
  (bind _returnvalue (`GameplayStatics.GetPlayerPawn` 0))
  (if (== OtherActor _returnvalue)
    (bind _asbp_player_vrcharacter (cast `/Game/VRGameContent/Player/BP_PlayerVRCharacter` _returnvalue))
    (`/Game/VRGameContent/Player/BP_PlayerVRCharacter.Set Draw Iteraction` _asbp_player_vrcharacter true)))

(event `self.BoxCollision.OnComponentEndOverlap`
  (params (OverlappedComponent :type "PrimitiveComponent Object Reference") (OtherActor :type "Actor Object Reference") (OtherComp :type "PrimitiveComponent Object Reference") (OtherBodyIndex :type Integer))
  (bind _returnvalue (`GameplayStatics.GetPlayerPawn` 0))
  (if (== OtherActor _returnvalue)
    (bind _asbp_player_vrcharacter (cast `/Game/VRGameContent/Player/BP_PlayerVRCharacter` _returnvalue))
    (`/Game/VRGameContent/Player/BP_PlayerVRCharacter.Set Draw Iteraction` _asbp_player_vrcharacter false)))

(fn `UserConstructionScript`)